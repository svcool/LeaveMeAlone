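; GM_LeaveMeAlone is the game mode that runs the match countdown and shows the end screens.
; Two looping one-second timers start on BeginPlay: one decrements GameTime, the other polls the player's LMAHealthComponent for zero health.
; Death opens WBP_GameOver after a short delay, while time running out opens WBP_Finish unless that menu is already stored.
; A shared ViewPortMenu function creates the widget, shows the cursor and switches to UI-only input.
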(event `self.ReceiveBeginPlay`
  ;[1 1 1] Таймер
  (`|ExecutionSequence`
    (:`then_0`
      (bind _returnvalue (`KismetSystemLibrary.K2_SetTimerDelegate` (delegate `CustomEvent`) 1.0 true))
      (set `self.Game Timer Handle` _returnvalue))
    (:`then_1`
      (bind _returnvalue_2 (`KismetSystemLibrary.K2_SetTimerDelegate` (delegate `GameOver`) 1.0 true))
      (set `self.CallGameOverr` _returnvalue_2))))

(event `CustomEvent`
  ;[1 1 1] Таймер
  (bind _output_get (set `self.GameTime` (- (`self.GameTime`) 1)))
  (if (== _output_get 0)
    (`/Engine/EditorBlueprintResources/StandardMacros.IsValid` (stale `GameOver` _widgetobject)
      (:`Is Not Valid`
        (`KismetSystemLibrary.K2_ClearAndInvalidateTimerHandle` (`self.Game Timer Handle`))
        (`self.View Port Menu` "/Game/LeaveMeAlone/Widgets/UI/WBP_Finish.WBP_Finish_C")))))

(event `self.ReceiveTick`
  (params (DeltaSeconds :type "Float (single-precision)")))

(event `GameOver`
  (if (== (`LMAHealthComponent.GetHealth` (`self.GetComponentByClass` (`GameplayStatics.GetPlayerCharacter` 0) "/Script/LeaveMeAlone.LMAHealthComponent")) 0.0)
    (`KismetSystemLibrary.Delay` 1.0)
    (`KismetSystemLibrary.K2_ClearAndInvalidateTimerHandle` (`self.CallGameOverr`))
    (bind _widgetobject (`self.View Port Menu` "/Game/LeaveMeAlone/Widgets/UI/WBP_GameOver.WBP_GameOver_C"))))

(fn `UserConstructionScript`)

(fn `View Port Menu`
  (params (WBP :type "UserWidget Class Reference"))
  (returns (widgetObject :type "UserWidget Object Reference"))
  (locals (NewLocalVar :type "UserWidget Object Reference"))
  (bind _returnvalue (`GameplayStatics.GetPlayerController` 0))
  (bind _returnvalue_2 (`|CreateWidget` WBP))
  (bind _output_get (set `local.NewLocalVar` _returnvalue_2))
  (`UserWidget.AddToViewport` _output_get 0)
  (set `PlayerController.bShowMouseCursor` true _returnvalue)
  (`WidgetBlueprintLibrary.SetInputMode_UIOnlyEx` _returnvalue _output_get)
  (return _returnvalue_2))